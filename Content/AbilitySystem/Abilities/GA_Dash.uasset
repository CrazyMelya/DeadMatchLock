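; Gameplay ability that dashes a DMLCharacter along its last movement input direction.
; On activation, only the locally controlled path proceeds; it ends if there is no movement input and cancels if the avatar is not a DMLCharacter.
; The Push event commits the ability and runs an additive, gravity-enabled constant-force root motion task, keeping its velocity on finish and then ending the ability.
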(event Custom|Push
  (params (DashDirection :type Vector))
  (Ability|CommitAbility)
  (Ability|Tasks|ApplyRootMotionConstantForce "Dash" DashDirection 1e+03 0.0 true 0 "MaintainLastRootMotionVelocity" "0, 0, 0" 0.0 true
    (:OnFinish
      (Ability|EndAbility))))

(event Ability|EventActivateAbility
  (Pawn|IsLocallyControlled
    (:True
      (bind _asdmlcharacter (Utilities|Casting|CastToDMLCharacter (Ability|GetAvatarActorfromActorInfo))
        (:then
          (if (Utilities|Operators|NotEqual(!=) :A (Class|Pawn|GetLastMovementInputVector _asdmlcharacter))
            (CallFunction|Push (Class|Pawn|GetLastMovementInputVector _asdmlcharacter))
            (else
              (Ability|EndAbility))))
        (:CastFailed
          (Ability|CancelAbility))))))