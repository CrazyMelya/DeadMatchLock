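; Player controller for the menu that handles session hosting, match start and session invites.
; CreateSession makes an Advanced Sessions session flagged as dedicated, then opens the game map on success.
; StartMatch forwards lobby data to another StartMatch call.
; Both invite received and invite accepted events show an invite widget built from the inviter and search result, with received also printing a debug message.
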(event Custom|StartMatch
  (params (LobbyData :type Lobby%20Data%20Structure))
  (bind _returnvalue (Class|LobbyManager|Get self))
  (Class|LobbyManager|StartMatch _returnvalue LobbyData))

(event Custom|CreateSession
  (|AdvancedSession 0 self 100 4 false true true true true false false false true false true
    (:OnSuccess
      (Game|OpenLevel(byObjectReference) "/Game/Maps/GameMap.GameMap" false))))

(event EventOnSessionInviteReceived
  (params (PersonInviting :type BP%20Unique%20Net%20Id%20Structure) (SearchResult :type Blueprint%20Session%20Result%20Structure%20%28by%20ref%29))
  (Development|PrintString "Invite Received")
  (bind _returnvalue (UserInterface|CreateWidget "/Game/Widgets/WBP_Invite.WBP_Invite_C" (Game|GetPlayerController 0) (stale EventOnSessionInviteAccepted PersonInvited) (stale EventOnSessionInviteAccepted SearchResult)))
  (UserInterface|Viewport|AddtoViewport _returnvalue 0))

(event EventOnSessionInviteAccepted
  (params (PersonInvited :type BP%20Unique%20Net%20Id%20Structure) (SearchResult :type Blueprint%20Session%20Result%20Structure%20%28by%20ref%29))
  (bind _returnvalue (UserInterface|CreateWidget "/Game/Widgets/WBP_Invite.WBP_Invite_C" (Game|GetPlayerController 0) PersonInvited SearchResult))
  (UserInterface|Viewport|AddtoViewport _returnvalue 0))

(fn ConstructionScript)