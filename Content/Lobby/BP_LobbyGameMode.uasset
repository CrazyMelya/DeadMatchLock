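; Lobby game mode that handles shutting down a multiplayer lobby through a CloseLobby event.
; On the server, it calls DestroySession for every controller in Players except player 0, then for player 0 itself.
; When that last call succeeds, it opens the MainMenu level.
; A KickPlayer call with a "Lobby was closed" reason is present but never runs.
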(event Custom|CloseLobby
  (bind _returnvalue (Game|GetPlayerController 0))
  (if (Networking|IsServer)
    (for _array_element (Variables|Default|GetPlayers)
      (if (!= _array_element _returnvalue)
        (|DestroySession _array_element)))
    (|DestroySession _returnvalue
      (:OnSuccess
        (Game|OpenLevel(byObjectReference) "/Game/Maps/MainMenu.MainMenu")))))

(fn ConstructionScript)