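; BP_LobbyPlayerPlatform is a lobby slot that displays a player's character or, while free, a button for opening the friend list.
; On the server, it links the button widget to itself and finds the BP_FriendList actor.
; Opening the list moves that actor onto the platform.
; Spawning stores the controller, creates a BP_LobbyCharacter and hides the button and any list located there; clearing removes the character and restores the button.
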(event Custom|Spawn%20Character
  (params (Controller :type Player%20Controller%20Object%20Reference))
  (Variables|Default|SetPlayer Controller)
  (Utilities|IsValid (Variables|Default|GetCharacter)
    (:Is%20Valid
      (Actor|DestroyActor (Variables|Default|GetCharacter)))
    (:Is%20Not%20Valid
      _))
  (bind _returnvalue (Game|SpawnActorfromClass "/Game/Lobby/BP_LobbyCharacter.BP_LobbyCharacter_C" (Transformation|GetWorldTransform (Variables|Default|GetPlayerSpawnTransform)) "AdjustIfPossibleButAlwaysSpawn" "MultiplyWithRoot" 0 0))
  (Variables|Default|SetCharacter _returnvalue)
  (Rendering|SetVisibility (Variables|Default|GetFriendListButton) false false)
  (if (Utilities|Operators|EqualEqual (Transformation|GetWorldLocation (Variables|Default|GetPlayerSpawnTransform)) (Transformation|GetActorLocation (Variables|Default|GetFriendList)) 1.0)
    (Default|Show (Variables|Default|GetFriendList) false)))

(event Custom|Clear
  (Variables|Default|SetPlayer 0)
  (Rendering|SetVisibility (Variables|Default|GetFriendListButton) true false)
  (Utilities|IsValid (Variables|Default|GetCharacter)
    (:Is%20Valid
      (Actor|DestroyActor (Variables|Default|GetCharacter))
      (Variables|Default|SetCharacter 0))))

(event EventBeginPlay
  (CallFunction|SetUpServer))

(fn ConstructionScript)

(fn GetPlayerController
  (return (Variables|Default|GetPlayer)))

(fn ShowFriendList
  (params (bShow :type Boolean))
  (Widget|SetVisibility (UserInterface|GetWidget (Variables|Default|GetFriendListButton)) (select bShow "Collapsed" "Visible"))
  (if bShow
    (Transformation|SetActorLocation (Variables|Default|GetFriendList) (Transformation|GetWorldLocation (Variables|Default|GetPlayerSpawnTransform)) false false)
    (Default|Show (Variables|Default|GetFriendList) true self)))

(fn SetUpServer
  (if (Networking|IsServer)
    (bind _outactors (Actor|GetAllActorsOfClass "/Game/Lobby/BP_FriendList.BP_FriendList_C"))
    (Variables|Default|SetFriendList (Utilities|Array|Get(acopy) _outactors))
    (bind _aswbp_show_lobby_friend_list_button (Utilities|Casting|CastToWBP_ShowLobbyFriendListButton (UserInterface|GetWidget (Variables|Default|GetFriendListButton))))
    (Variables|/Game/Widgets/Lobby/WBP_ShowLobbyFriendListButton.WBP_ShowLobbyFriendListButton_C|SetLobbyPlayerPlatform _aswbp_show_lobby_friend_list_button self)
    (Rendering|SetVisibility (Variables|Default|GetFriendListButton) true false)))