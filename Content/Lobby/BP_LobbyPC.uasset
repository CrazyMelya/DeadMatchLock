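; Lobby player controller that gives the local player the lobby UI and holds their lobby info, including name and ready status.
; On BeginPlay the local controller shows the cursor, creates the lobby widget and submits the player's name.
; The server-named name and ready-toggle events edit the info struct, then pass the controller to BP_LobbyGM to update.
; StartMatch is an empty event.
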(event Custom|UpdateLobbyInfo
  (bind _asbp_lobby_gm (Utilities|Casting|CastToBP_LobbyGM (Game|GetGameMode)))
  (Default|UpdatePlayerLobbyInfo _asbp_lobby_gm self))

(event Custom|SetPlayername_Server
  (params (PlayerName :type Text))
  (Utilities|Struct|SetmembersinS_PlayerLobbyInfo (Variables|Default|GetPlayerLobbyInfo) PlayerName)
  (CallFunction|UpdateLobbyInfo))

(event Custom|ToggleReadyStatus_Server
  (Utilities|Struct|SetmembersinS_PlayerLobbyInfo (Variables|Default|GetPlayerLobbyInfo) (not (Utilities|Struct|BreakS_PlayerLobbyInfo (Variables|Default|GetPlayerLobbyInfo))))
  (CallFunction|UpdateLobbyInfo))

(event Custom|StartMatch)

(event EventBeginPlay
  (CallFunction|SetUp))

(fn ConstructionScript)

(fn SetUp
  (if (Pawn|IsLocalPlayerController)
    (Variables|Default|SetbShowMouseCursor true)
    (Input|SetInputModeGameandUI self 0 "DoNotLock" false false)
    (bind _returnvalue (UserInterface|CreateWidget "/Game/Widgets/Lobby/WBP_LobbyUI.WBP_LobbyUI_C"))
    (bind _output_get (Variables|Default|SetLobbyUI _returnvalue))
    (UserInterface|Viewport|AddtoViewport _output_get 0)
    (CallFunction|SetPlayernameServer (Utilities|Text|ToText(String) (Class|AdvancedSessionsLibrary|GetPlayerName self)))))