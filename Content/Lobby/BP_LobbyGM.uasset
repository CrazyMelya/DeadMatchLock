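; Lobby game mode that seats joining players on tagged BP_LobbyPlayerPlatform actors, each spawning that player's character.
; BeginPlay orders platforms by index tag and seats players who logged in earlier; later logins take the first free platform.
; A controller-to-platform map drives clearing on logout and pushing name and ready state to lobby characters.
; It also provides an all-players-ready check and a kick function.
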(event EventBeginPlay
  (CallFunction|SetUpPlatforms)
  (CallFunction|SetUpFirstPlayers))

(event EventPostLogin
  (params (NewPlayer :type Player%20Controller%20Object%20Reference))
  (CallFunction|AddNewPlayer NewPlayer))

(event EventOnLogout
  (params (ExitingController :type Controller%20Object%20Reference))
  (CallFunction|RemovePlayer ExitingController))

(fn ConstructionScript)

(fn SetUpPlatforms
  (bind _outactors (Actor|GetAllActorsOfClass "/Game/Lobby/BP_LobbyPlayerPlatform.BP_LobbyPlayerPlatform_C"))
  (for (_ _array_index) _outactors
    (bind _outactors_2 (Actor|GetAllActorsOfClasswithTag "/Game/Lobby/BP_LobbyPlayerPlatform.BP_LobbyPlayerPlatform_C" (Utilities|String|StringToName (Utilities|String|ToString(Integer) _array_index))))
    (Utilities|Array|Add (Variables|Default|GetPlayerPlatforms) (Utilities|Array|Get(acopy) _outactors_2)))
  (Variables|Default|SetbPlaformsSetupDone true))

(fn AddNewPlayer
  (params (New%20Player :type Player%20Controller%20Object%20Reference%20%28by%20ref%29))
  (if (Variables|Default|GetbPlaformsSetupDone)
    (for _array_element (Variables|Default|GetPlayerPlatforms)
      (bind _output_get (LocalVariables|SetCurrentPlatform _array_element))
      (if (not (Utilities|IsValid (Default|GetPlayerController _output_get)))
        (Default|SpawnCharacter (LocalVariables|GetCurrentPlatform) New%20Player)
        (Utilities|Map|Add (Variables|Default|GetPlayersMap) New%20Player (LocalVariables|GetCurrentPlatform))
        (return)))
    (else
      (Utilities|Map|Add (Variables|Default|GetPlayersMap) New%20Player 0))))

(fn SetUpFirstPlayers
  (bind _keys (Utilities|Map|Keys (Variables|Default|GetPlayersMap)))
  (for (_array_element _array_index) _keys
    (bind _output_get (LocalVariables|SetCurrentPlayer _array_element))
    (Utilities|Map|Add (Variables|Default|GetPlayersMap) _output_get (Utilities|Array|Get(acopy) (Variables|Default|GetPlayerPlatforms) _array_index))
    (Default|SpawnCharacter (Utilities|Array|Get(acopy) (Variables|Default|GetPlayerPlatforms) _array_index) (LocalVariables|GetCurrentPlayer))))

(fn RemovePlayer
  (params (Player :type Object%20Object%20Reference))
  (bind _asplayer_controller (Utilities|Casting|CastToPlayerController Player))
  (Default|Clear (.Value (Utilities|Map|Find (Variables|Default|GetPlayersMap) _asplayer_controller)))
  (Utilities|Map|Remove (Variables|Default|GetPlayersMap) _asplayer_controller))

(fn UpdatePlayerLobbyInfo
  (params (Controller :type Player%20Controller%20Object%20Reference))
  (bind _asbp_lobby_pc (Utilities|Casting|CastToBP_LobbyPC Controller))
  (bind _playerlobbyinfo (Variables|/Game/Lobby/BP_LobbyPC.BP_LobbyPC_C|GetPlayerLobbyInfo _asbp_lobby_pc))
  (bind (_playername _bready) (Utilities|Struct|BreakS_PlayerLobbyInfo _playerlobbyinfo))
  (Default|UpdateLobbyInfo (Variables|/Game/Lobby/BP_LobbyPlayerPlatform.BP_LobbyPlayerPlatform_C|GetCharacter (.Value (Utilities|Map|Find (Variables|Default|GetPlayersMap) Controller))) (Utilities|Struct|MakeS_PlayerLobbyInfo Controller _playername _bready (Variables|/Script/Engine.Controller|GetPlayerState _asbp_lobby_pc))))

(fn CheckAllPlayersReady
  (bind _keys (Utilities|Map|Keys (Variables|Default|GetPlayersMap)))
  (for _array_element _keys
    (bind _asbp_lobby_pc (Utilities|Casting|CastToBP_LobbyPC _array_element))
    (if (not (Utilities|Struct|BreakS_PlayerLobbyInfo (Variables|/Game/Lobby/BP_LobbyPC.BP_LobbyPC_C|GetPlayerLobbyInfo _asbp_lobby_pc)))
      (return false)))
  (return true))

(fn KickPlayer
  (params (PlayerToKick :type Player%20Controller%20Object%20Reference))
  (Class|AdvancedSessionsLibrary|KickPlayer PlayerToKick))